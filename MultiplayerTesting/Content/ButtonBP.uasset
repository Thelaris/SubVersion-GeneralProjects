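; Multiplayer push button that a player uses while overlapping it, announcing that player's name.
; On the authority, it binds PressButtonEvent to the MultiplayerGamemode's use dispatcher, checks pawn overlap, passes PlayerName to CallChangeText, nudges itself along X for a second, then prints the name.
; Box overlap toggles input for player controller 0.
; GameState-based location syncing, a timeline move and DoOnce resets remain as largely disconnected leftovers.
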(event OnComponentEndOverlap(Box)
  (params (OtherActor :type Actor%20Object%20Reference) (OtherComp :type Primitive%20Component%20Object%20Reference) (OtherBodyIndex :type Integer))
  (Input|DisableInput (Game|GetPlayerController 0)))

(event OnComponentBeginOverlap(Box)
  (params (OtherActor :type Actor%20Object%20Reference) (OtherComp :type Primitive%20Component%20Object%20Reference) (OtherBodyIndex :type Integer) (bFromSweep :type Boolean) (SweepResult :type Hit%20Result%20Structure%20%28by%20ref%29))
  (Input|EnableInput (Game|GetPlayerController 0)))

(event Custom|SetActorLocation
  (params (ActorLocation :type Vector))
  (bind _asmultiplayer_game_state (Utilities|Casting|CastToMultiplayerGameState (Game|GetGameState)))
  (bind _output_get (Variables|/Game/MultiplayerGameState.MultiplayerGameState_C|SetButtonLocation _asmultiplayer_game_state ActorLocation)))

(event Custom|MoveButtonEvent
  (bind _buttonvectortrack (Timeline|MoveButton Play)
    (:Update
      (CallFunction|SetActorLocation (+ _buttonvectortrack (Variables|Default|GetActorStartLocation))))
    (:Finished
      (bind _asmultiplayer_game_state (Utilities|Casting|CastToMultiplayerGameState (Game|GetGameState)))
      (Variables|/Game/MultiplayerGameState.MultiplayerGameState_C|SetButtonPressed _asmultiplayer_game_state false))))

(event Custom|PrintPlayer
  (Development|PrintString (Utilities|String|ToString(Text) (Variables|/Game/AnimStarterPack/Ue4ASP_Character.Ue4ASP_Character_C|GetPlayerName (stale Custom|PressButtonEvent _asue_4asp_character))) true true "(R=1.000000,G=0.000000,B=0.000000,A=1.000000)" 6e+01))

(event Custom|ResetButton)

(event Custom|SendToServer
  (bind _asmultiplayer_game_state (Utilities|Casting|CastToMultiplayerGameState (Game|GetGameState)))
  (Variables|/Game/MultiplayerGameState.MultiplayerGameState_C|SetButtonLocation _asmultiplayer_game_state (+ (Variables|Default|GetActorStartLocation) "10.000000, 0, 0"))
  (Variables|/Game/MultiplayerGameState.MultiplayerGameState_C|SetButtonPressed _asmultiplayer_game_state true))

(event Custom|ServerExecute)

(event Custom|PressButtonEvent
  (params (NewParam :type Player%20Controller%20BP%20Object%20Reference))
  (bind _returnvalue (Transformation|GetActorLocation))
  (if (Collision|IsOverlappingActor (Pawn|GetControlledPawn NewParam) :!class /Script/Engine.Actor)
    (Variables|Default|SetPlayerControllerRef NewParam)
    (Variables|Default|SetIsButtonPressed true)
    (bind _asue_4asp_character (Utilities|Casting|CastToUe4ASP_Character (Pawn|GetControlledPawn (Variables|Default|GetPlayerControllerRef))))
    (Default|CallChangeText (Variables|/Game/AnimStarterPack/Ue4ASP_Character.Ue4ASP_Character_C|GetPlayerName _asue_4asp_character))
    (Transformation|SetActorLocation (+ _returnvalue "10.000000, 0, 0") false false)
    (Utilities|FlowControl|Delay 1.0)
    (Transformation|SetActorLocation (- _returnvalue "10.000000, 0, 0") false false)
    (Variables|Default|SetIsButtonPressed false)
    (CallFunction|PrintPlayer)))

(event Custom|ResetDoOnce)

(event Custom|ResetDoOnceUse
  (bind _returnvalue (Transformation|GetActorLocation))
  (Utilities|FlowControl|DoOnce false ; enters at Reset
    (:Completed
      (Variables|Default|SetActorLocation (+ _returnvalue "10.000000, 0, 0"))
      (Utilities|FlowControl|Delay 2.0)
      (Variables|Default|SetActorLocation (- _returnvalue "10.000000, 0, 0"))
      (CallFunction|ResetDoOnceUse))))

(event EventBeginPlay)

(event EventActorBeginOverlap
  (params (OtherActor :type Actor%20Object%20Reference)))

(event EventTick
  (params (DeltaSeconds :type Float%20%28single-precision%29)))

(event EventBeginPlay
  (Networking|SwitchHasAuthority
    (:Authority
      (bind _asmultiplayer_gamemode (Utilities|Casting|CastToMultiplayerGamemode (Game|GetGameMode)))
      (EventDispatchers|BindEventtoUseDPfromServer _asmultiplayer_gamemode (delegate Custom|PressButtonEvent)))))

(event Input|ActionEvents|InputActionUseKey
  (params (Key :type Key%20Structure :default "AnyKey")))

(fn ConstructionScript)

(fn ActivateF)