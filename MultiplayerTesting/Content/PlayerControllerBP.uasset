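; Player controller Blueprint that creates the local player's HUD and relays the Use key input.
; On BeginPlay it waits briefly, then, for the local controller only, creates the HUD widget, stores it and adds it to the viewport.
; Pressing UseKey calls CallUseKeyOnServer, named as a server-side event, which fires DPPCUseKey with this controller as the argument.
; The ConstructHUD event is an empty stub.
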(event Custom|ConstructHUD)

(event Custom|CallUseKeyOnServer
  (bind _output_get (Variables|Default|SetPlayerController self))
  (Default|CallDPPCUseKey _output_get))

(event EventBeginPlay
  (Utilities|FlowControl|Delay 1.0)
  (if (Pawn|IsLocalController)
    (bind _returnvalue (UserInterface|CreateWidget "/Game/HUD.HUD_C" self))
    (bind _output_get (Variables|Default|SetHUDReference _returnvalue))
    (UserInterface|Viewport|AddtoViewport _output_get 0)))

(event EventTick
  (params (DeltaSeconds :type Float%20%28single-precision%29)))

(event Input|ActionEvents|InputActionUseKey
  (params (Key :type Key%20Structure :default "AnyKey"))
  (:Pressed
    (CallFunction|CallUseKeyonServer)))

(fn ConstructionScript)